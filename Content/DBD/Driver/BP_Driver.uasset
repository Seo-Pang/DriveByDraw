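; BP_Driver is a driver actor that owns a card deck and links it to the game's UI and monster spawning.
; On BeginPlay it constructs and initializes a DeckSet, then caches the PlayerHand widget from the UIManager tagged "UI".
; A lookup returns that manager's ActionQueue, additionally filtering by the misspelled "Manger" tag.
; SpawnMonster spawns a given class at the driver's transform, hosted here because spawning failed elsewhere.
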(event EventBeginPlay
  (bind _returnvalue (Game|ConstructObjectfromClass (Variables|Default|GetDeckSet) self))
  (bind _output_get (Variables|Default|SetDeck _returnvalue))
  (Class|Deck|InitDeck _output_get)
  (CallFunction|SetOwnHandWidget))

(event Collision|EventActorBeginOverlap
  (params (OtherActor :type Actor%20Object%20Reference)))

(event EventTick
  (params (DeltaSeconds :type Float%20%28single-precision%29)))

(fn ConstructionScript)

(fn FindActionQueueWidget
  (bind _outactors (Actor|GetAllActorsOfClasswithTag "/Game/DBD/Manger/UIManager.UIManager_C" "Manger"))
  (for _array_element _outactors
    (if (Actor|ActorHasTag _array_element "UI")
      (return (Variables|/Game/DBD/Manger/UIManager.UIManager_C|GetActionQueue _array_element)))))

(fn SetOwnHandWidget
  (bind _outactors (Actor|GetAllActorsOfClass "/Game/DBD/Manger/UIManager.UIManager_C"))
  (for _array_element _outactors
    (if (Actor|ActorHasTag _array_element "UI")
      (Development|PrintString "ss")
      (bind _output_get (Variables|Default|SetHandWidget (Variables|/Game/DBD/Manger/UIManager.UIManager_C|GetPlayerHand _array_element)))
      (Utilities|IsValid _output_get
        (:Is%20Valid
          _)
        (:Is%20Not%20Valid
          (Development|PrintString "Not to Hand")))
      (return)
      (else
        (Development|PrintString "Not to Driver")))))

(fn SpawnMonster
  (params (MonsterClass :type Monster%20Class%20Reference))
  ;[1 1 1] 이상하게 다른 곳에서 하면 스폰이 안되어서 여기서 합니다.
  (bind _returnvalue (Game|SpawnActorfromClass MonsterClass (Transformation|GetActorTransform) "AlwaysSpawn" 0 0))
  (return _returnvalue))