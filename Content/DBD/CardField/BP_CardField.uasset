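; BP_CardField is a card-battle field slot that turns cards dropped on it into queued actions for its owner.
; On BeginPlay it finds the card manager, the UI manager's action queue and the team's tagged driver, assigning that driver's hand widget.
; DragOnCard checks mana, builds a spawn action for empty slots or attack action for occupied ones, enqueues it and deducts cost.
; A helper adds monster-owned attack cards to the owner's hand.
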(event EventBeginPlay
  (Utilities|FlowControl|Sequence
    (:then_0
      (Utilities|FlowControl|Delay 0.01)
      ;[1 1 1] 카드 매니저 불러오기
      (bind _outactors (Actor|GetAllActorsOfClass "/Game/DBD/Manger/CardManager.CardManager_C"))
      (for _array_element _outactors
        (Variables|Default|SetCardManger _array_element)))
    (:then_1
      (Utilities|FlowControl|Delay 0.01)
      ;[1 1 1] 액션  큐 불러오기
      (bind _outactors_2 (Actor|GetAllActorsOfClass "/Game/DBD/Manger/UIManager.UIManager_C"))
      (for _array_element_2 _outactors_2
        (Variables|Default|SetActionQueue (Variables|/Game/DBD/Manger/UIManager.UIManager_C|GetActionQueue _array_element_2))))
    (:then_2
      (Utilities|FlowControl|Delay 0.01)
      (if (Variables|/Script/DriveByDraw.Driver|GetMyTeam (Variables|Default|GetFieldOwner))
        (bind _outactors_3 (Actor|GetAllActorsOfClasswithTag "/Game/DBD/Driver/BP_Driver.BP_Driver_C" "Player"))
        (for _array_element_3 _outactors_3
          (bind _output_get (Variables|Default|SetOwned _array_element_3))
          (Variables|/Game/DBD/Driver/BP_Driver.BP_Driver_C|SetHandWidget _output_get (Variables|/Game/DBD/Manger/UIManager.UIManager_C|GetPlayerHand _array_element_2)))
        (else
          (bind _outactors_4 (Actor|GetAllActorsOfClasswithTag "/Game/DBD/Driver/BP_Driver.BP_Driver_C" "Enemy"))
          (for _array_element_4 _outactors_4
            (bind _output_get_2 (Variables|Default|SetOwned _array_element_4))
            (Variables|/Game/DBD/Driver/BP_Driver.BP_Driver_C|SetHandWidget _output_get_2 (Variables|/Game/DBD/Manger/UIManager.UIManager_C|GetPlayerHand _array_element_2))))))))

(event Collision|EventActorBeginOverlap
  (params (OtherActor :type Actor%20Object%20Reference)))

(event EventTick
  (params (DeltaSeconds :type Float%20%28single-precision%29)))

(fn ConstructionScript)

(fn DragonCard
  (params (DragCard :type Card%20Object%20Reference))
  (bind _fieldowner (Variables|Default|GetFieldOwner))
  (bind _castable (CallFunction|CastbyCost DragCard))
  (if _castable
    (bind (_action _issuccess) (CallFunction|CreateAction DragCard))
    (if _issuccess
      (Utilities|IsValid _action
        (:Is%20Valid
          (Default|EnqueueAction (Variables|Default|GetActionQueue) _action)
          (Variables|/Script/DriveByDraw.Driver|SetMana _fieldowner (- (Variables|/Script/DriveByDraw.Driver|GetMana _fieldowner) (Math|Conversions|ToFloat(Byte) (Variables|/Script/DriveByDraw.Card|Getcost DragCard))))
          (return true))
        (:Is%20Not%20Valid
          _)))
    (Development|PrintString "액션이 생성되지 않았습니다." true true "(R=1.000000,G=0.042180,B=0.000000,A=1.000000)")
    (return false)
    (else
      (if (Variables|Default|GetMyTeam)
        (Development|PrintString "마나가 부족합니다." true true "(R=0.076689,G=0.241337,B=1.000000,A=1.000000)"))
      (return false))))

(fn ActMonsterCard
  (params (MonsterCard :type Card%20Object%20Reference))
  (bind _returnvalue (Game|ConstructObjectfromClass "/Script/DriveByDraw.ActionSpawn" (Variables|Default|GetFieldOwner)))
  (bind _output_get (Variables|/Script/DriveByDraw.Action|SetActingField _returnvalue self))
  (Variables|/Script/DriveByDraw.Action|SetActionOwner _returnvalue (Variables|/Script/DriveByDraw.CardField|GetFieldOwner _output_get))
  (Variables|/Script/DriveByDraw.ActionSpawn|SetMonsterSet _returnvalue (Variables|/Script/DriveByDraw.Card|GetCardMonster MonsterCard))
  (return _returnvalue))

(fn ActAttackCard
  (params (AttackCard :type Card%20Object%20Reference))
  (bind _castmonster (Variables|/Script/DriveByDraw.Card|GetCastMonster AttackCard))
  (bind _returnvalue (Game|ConstructObjectfromClass "/Script/DriveByDraw.ActionAttack" (Variables|Default|GetFieldOwner)))
  (bind _output_get (Variables|/Script/DriveByDraw.Action|SetActingField _returnvalue self))
  (Variables|/Script/DriveByDraw.Action|SetActionOwner _returnvalue (Variables|/Script/DriveByDraw.CardField|GetFieldOwner _output_get))
  (Utilities|IsValid _castmonster
    (:Is%20Valid
      (Variables|/Script/DriveByDraw.Action|SetCastingMonster _returnvalue _castmonster)
      (Variables|/Script/DriveByDraw.Action|SetTargettingMonster _returnvalue (Variables|Default|GetSettingMonster))
      (return _returnvalue))
    (:Is%20Not%20Valid
      (Development|PrintString (Utilities|GetObjectName _castmonster)))))

(fn CreateAction
  (params (card :type Card%20Object%20Reference))
  (bind _settingmonster (Variables|Default|GetSettingMonster))
  (switch Utilities|FlowControl|Switch|SwitchonCardType (Variables|/Script/DriveByDraw.Card|Gettype card)
    (:Card
      (Development|PrintString "설정이 되어 있지 않은 카드입니다.")
      (return 0 false))
    (:MonsterCard
      (Utilities|IsValid _settingmonster
        (:Is%20Valid
          (Development|PrintString "이미 몬스터가 있습니다." true true "(R=1.000000,G=0.142871,B=0.000000,A=1.000000)")
          (return 0 false))
        (:Is%20Not%20Valid
          (bind _spawnaction (CallFunction|ActMonsterCard card))
          (return _spawnaction true))))
    (:AttackCard
      (Utilities|IsValid _settingmonster
        (:Is%20Valid
          (bind _actionattack (CallFunction|ActAttackCard card))
          (return _actionattack true))
        (:Is%20Not%20Valid
          (Development|PrintString "몬스터가 존재하지 않습니다.")
          (return 0 false))))))

(fn CreateAttackCard
  (params (AttackingMonster :type Monster%20Object%20Reference))
  (bind _fieldowner (Variables|Default|GetFieldOwner))
  (bind _asbp_driver (Utilities|Casting|CastToBP_Driver _fieldowner))
  (bind _handwidget (Variables|/Game/DBD/Driver/BP_Driver.BP_Driver_C|GetHandWidget _asbp_driver))
  (bind _returnvalue (Game|ConstructObjectfromClass "/Game/DBD/Card/AttackCard.AttackCard_C" _fieldowner))
  (Variables|/Game/DBD/Card/AttackCard.AttackCard_C|SetOwnMonster _returnvalue AttackingMonster)
  (Default|AddCard _handwidget (Variables|/Game/DBD/UI/Blueprint/WBP_Hand.WBP_Hand_C|GetHandBox _handwidget) _returnvalue))

(fn CastbyCost
  (params (card :type Card%20Object%20Reference))
  (return (not (> (Math|Conversions|ToFloat(Byte) (Variables|/Script/DriveByDraw.Card|Getcost card)) (Variables|/Script/DriveByDraw.Driver|GetMana (Variables|Default|GetFieldOwner))))))