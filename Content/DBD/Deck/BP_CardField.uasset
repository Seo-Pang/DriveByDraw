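; BP_CardField is a card field that holds one monster and turns cards dragged onto it into queued actions.
; BeginPlay finds the CardManager, the UIManager's ActionQueue and the team-tagged BP_Driver, assigning its hand widget.
; DragOnCard enqueues an ActionSpawn for monster cards on an empty field, or an ActionAttack targeting the occupying monster.
; SpawnMob resolves a monster class through CardManager lookups and spawns it via the Player-tagged driver.
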(event EventBeginPlay
  (Utilities|FlowControl|Sequence
    (:then_0
      (Utilities|FlowControl|Delay 0.01)
      ;[1 1 1] 카드 매니저 불러오기
      (bind _outactors (Actor|GetAllActorsOfClass "/Game/DBD/Manger/CardManager.CardManager_C"))
      (for _array_element _outactors
        (Variables|Default|SetCardManger _array_element)))
    (:then_1
      (Utilities|FlowControl|Delay 0.01)
      ;[1 1 1] 액션  큐 불러오기
      (bind _outactors_2 (Actor|GetAllActorsOfClass "/Game/DBD/Manger/UIManager.UIManager_C"))
      (for _array_element_2 _outactors_2
        (Variables|Default|SetActionQueue (Variables|/Game/DBD/Manger/UIManager.UIManager_C|GetActionQueue _array_element_2))))
    (:then_2
      (Utilities|FlowControl|Delay 0.01)
      (if (Variables|/Script/DriveByDraw.Driver|GetMyTeam (Variables|Default|GetFieldOwner))
        (bind _outactors_3 (Actor|GetAllActorsOfClasswithTag "/Game/DBD/Driver/BP_Driver.BP_Driver_C" "Player"))
        (for _array_element_3 _outactors_3
          (bind _output_get (Variables|Default|SetOwned _array_element_3))
          (Variables|/Game/DBD/Driver/BP_Driver.BP_Driver_C|SetHandWidget _output_get (Variables|/Game/DBD/Manger/UIManager.UIManager_C|GetPlayerHand _array_element_2)))
        (else
          (bind _outactors_4 (Actor|GetAllActorsOfClasswithTag "/Game/DBD/Driver/BP_Driver.BP_Driver_C" "Enemy"))
          (for _array_element_4 _outactors_4
            (bind _output_get_2 (Variables|Default|SetOwned _array_element_4))
            (Variables|/Game/DBD/Driver/BP_Driver.BP_Driver_C|SetHandWidget _output_get_2 (Variables|/Game/DBD/Manger/UIManager.UIManager_C|GetPlayerHand _array_element_2))))))))

(event Collision|EventActorBeginOverlap
  (params (OtherActor :type Actor%20Object%20Reference)))

(event EventTick
  (params (DeltaSeconds :type Float%20%28single-precision%29)))

(fn ConstructionScript)

(fn DragonCard
  (params (DragCard :type Card%20Object%20Reference))
  (bind _action (CallFunction|CreateAction DragCard))
  (Utilities|IsValid _action
    (:Is%20Valid
      (Default|EnqueueAction (Variables|Default|GetActionQueue) _action))
    (:Is%20Not%20Valid
      (Development|PrintString "액션이 생성되지 않았습니다.")))
  (return))

(fn SpawnMob
  (params (MonsterID :type Byte))
  (bind _cardmanger (Variables|Default|GetCardManger))
  (bind _cardmanger_2 (Variables|Default|GetCardManger))
  (bind _monstertable (Variables|/Game/DBD/Manger/CardManager.CardManager_C|GetMonsterTable _cardmanger))
  (bind _monsterclass (Variables|/Game/DBD/Manger/CardManager.CardManager_C|GetMonsterClass _cardmanger_2))
  (bind (_value _returnvalue) (Utilities|Map|Find _monstertable MonsterID))
  (bind (_value_2 _returnvalue_2) (Utilities|Map|Find _monsterclass _value))
  (bind _outactors (Actor|GetAllActorsOfClasswithTag "/Game/DBD/Driver/BP_Driver.BP_Driver_C" "Player"))
  (if (and _returnvalue _returnvalue_2)
    (bind _monster (Default|SpawnMonster _outactors _value_2))
    (bind _output_get (Variables|Default|SetSettingMonster _monster))
    (return _output_get)
    (else
      (Development|PrintString "Error(SpawnNotTable)")
      (return 0))))

(fn ActMonsterCard
  (params (MonsterCard :type Card%20Object%20Reference))
  (bind _returnvalue (Game|ConstructObjectfromClass "/Script/DriveByDraw.ActionSpawn" (Variables|Default|GetFieldOwner)))
  (bind _output_get (Variables|/Script/DriveByDraw.Action|SetActingField _returnvalue self))
  (Variables|/Script/DriveByDraw.Action|SetActionOwner _returnvalue (Variables|/Script/DriveByDraw.CardField|GetFieldOwner _output_get))
  (Variables|/Script/DriveByDraw.ActionSpawn|SetMonsterSet _returnvalue (Variables|/Script/DriveByDraw.Card|GetCardMonster MonsterCard))
  (return _returnvalue))

(fn ActAttackCard
  (params (AttackCard :type Card%20Object%20Reference))
  (bind _returnvalue (Game|ConstructObjectfromClass "/Script/DriveByDraw.ActionAttack" (Variables|Default|GetFieldOwner)))
  (bind _output_get (Variables|/Script/DriveByDraw.Action|SetActingField _returnvalue self))
  (Variables|/Script/DriveByDraw.Action|SetActionOwner _returnvalue (Variables|/Script/DriveByDraw.CardField|GetFieldOwner _output_get))
  (Variables|/Script/DriveByDraw.Action|SetCastingMonster _returnvalue (Variables|/Script/DriveByDraw.Card|GetCastMonster AttackCard))
  (Variables|/Script/DriveByDraw.Action|SetTargettingMonster _returnvalue (Variables|Default|GetSettingMonster))
  (return _returnvalue))

(fn CreateAction
  (params (card :type Card%20Object%20Reference))
  (bind _settingmonster (Variables|Default|GetSettingMonster))
  (switch Utilities|FlowControl|Switch|SwitchonCardType (Variables|/Script/DriveByDraw.Card|Gettype card)
    (:Card
      (Development|PrintString "설정이 되어 있지 않은 카드입니다."))
    (:MonsterCard
      (Utilities|IsValid _settingmonster
        (:Is%20Valid
          (Development|PrintString "이미 몬스터가 있습니다." true true "(R=1.000000,G=0.142871,B=0.000000,A=1.000000)")
          (return 0))
        (:Is%20Not%20Valid
          (bind _spawnaction (CallFunction|ActMonsterCard card))
          (return _spawnaction))))
    (:AttackCard
      (Utilities|IsValid _settingmonster
        (:Is%20Valid
          (bind _actionattack (CallFunction|ActAttackCard card))
          (return _actionattack))
        (:Is%20Not%20Valid
          (Development|PrintString "몬스터가 존재하지 않습니다.")
          (return 0))))))